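; BP_ColorChangeObject1 is an object whose Cube mesh takes its color, roughness and metallic look from Blueprint variables.
; On BeginPlay it creates a dynamic instance of each Cube material, stores them in DynamicMaterials, then calls SetValues.
; SetValues pushes the variables to every stored instance, though the color's vector parameter name is None, unlike the named Roughness and Metallic parameters.
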(event Custom|SetValues
  (for _array_element (Variables|Default|GetDynamicMaterials)
    (Rendering|Material|SetVectorParameterValue _array_element "None" (Variables|Default|GetColor) :!class /Script/Engine.MaterialInstanceDynamic)
    (Rendering|Material|SetScalarParameterValue _array_element "Roughness" (Variables|Default|GetRoughness) :!class /Script/Engine.MaterialInstanceDynamic)
    (Rendering|Material|SetScalarParameterValue _array_element "Metallic" (Variables|Default|GetMetallic) :!class /Script/Engine.MaterialInstanceDynamic)))

(event EventBeginPlay
  (bind _cube (Variables|Default|GetCube))
  (for (_array_element _array_index) (Rendering|Material|GetMaterials _cube)
    (bind _returnvalue (Rendering|Material|CreateDynamicMaterialInstance _cube _array_index _array_element "None" :!class /Script/Engine.PrimitiveComponent))
    (Utilities|Array|SetArrayElem (Variables|Default|GetDynamicMaterials) _array_index _returnvalue true))
  (CallFunction|SetValues))

(fn ConstructionScript)